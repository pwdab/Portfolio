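; BP_Character is a character Blueprint for a knight that dithers its material based on follow-camera distance.
; BeginPlay hides the cape and hand-slot bones and creates a dynamic material instance.
; Tick converts camera-to-actor distance into a clamped DitherAlpha, applied only when locally controlled.
; OnDodge is empty, and leftover graphs for bone unhiding, timeline-driven turning and dodging, and HUD creation are disconnected and never run.
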(event `self.ReceiveBeginPlay`
  (`SkinnedMeshComponent.HideBoneByName` (`self.Mesh`) "Knight_Cape" "PBO_None")
  (`SkinnedMeshComponent.HideBoneByName` (`self.Mesh`) "handslot_l" "PBO_None")
  (`SkinnedMeshComponent.HideBoneByName` (`self.Mesh`) "handslot_r" "PBO_None")
  (bind _returnvalue (`PrimitiveComponent.CreateDynamicMaterialInstance` (`self.Mesh`) 0 "/Game/Characters/Adventurers/Knight/knight_material.knight_material" "None"))
  (set `self.Dynamic Material Instance` _returnvalue))

(event `self.ReceiveTick`
  (params (DeltaSeconds :type "Float (single-precision)"))
  (bind _output_get (set `self.Current Camera Distance` (`KismetMathLibrary.VSize` (- (`SceneComponent.K2_GetComponentLocation` (`self.FollowCamera`)) (`self.K2_GetActorLocation`)))))
  (if (< 0.0 _output_get)
    (if (`self.IsLocallyControlled`)
      (`MaterialInstanceDynamic.SetScalarParameterValue` (`self.Dynamic Material Instance`) "DitherAlpha" (`KismetMathLibrary.FClamp` (/ (- (`self.Current Camera Distance`) 100.0) 200.0))))))

(event `self.OnDodge`
  (params (LaunchVector :type "Vector Structure (by ref)")))

(fn `UserConstructionScript`)