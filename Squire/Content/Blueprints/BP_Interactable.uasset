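; BP_Interactable is an interactable actor with a sphere that toggles between active and inactive states.
; BeginPlay creates a dynamic material on the sphere and stores its Color parameter in BaseColor.
; Interact flips IsActive, prints the new state and recolors the sphere red when active or light grey when inactive.
; CanInteract always returns false, and Interact does not consult it.
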(event `self.ReceiveBeginPlay`
  (bind _returnvalue (`PrimitiveComponent.CreateDynamicMaterialInstance` (`self.Sphere`) 0 null "None"))
  (bind _returnvalue_2 (`MaterialInstanceDynamic.K2_GetVectorParameterValue` _returnvalue "Color"))
  (set `self.Base Color` _returnvalue_2))

(event `self.Interact`
  (params (CharacterInstigator :type "PS_Character Object Reference"))
  (if (`self.bIsActive`)
    (set `self.bIsActive` false)
    (`KismetSystemLibrary.PrintString` "Not Active")
    (bind _output_get (set `self.Base Color` (struct :`R` 0.9 :`G` 0.9 :`B` 0.9 :`A` 1.0)))
    (bind _returnvalue (`PrimitiveComponent.CreateDynamicMaterialInstance` (`self.Sphere`) 0 null "None"))
    (`MaterialInstanceDynamic.SetVectorParameterValue` _returnvalue "Color" _output_get)
    (else
      (set `self.bIsActive` true)
      (`KismetSystemLibrary.PrintString` "Active")
      (bind _output_get_2 (set `self.Base Color` (struct :`R` 0.9 :`A` 1.0)))
      (bind _returnvalue_2 (`PrimitiveComponent.CreateDynamicMaterialInstance` (`self.Sphere`) 0 null "None"))
      (`MaterialInstanceDynamic.SetVectorParameterValue` _returnvalue_2 "Color" _output_get_2))))

(fn `CanInteract`
  (params (CharacterInstigator :type "PS_Character Object Reference"))
  (returns (ReturnValue :type Boolean))
  (return false))

(fn `UserConstructionScript`)