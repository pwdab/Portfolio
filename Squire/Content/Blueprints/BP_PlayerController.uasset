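; Player controller that routes debug and menu hotkeys to BP_HUD and can end the current online session.
; BeginPlay polls on a short delay until the HUD casts to BP_HUD, then caches it; UpdateHUD refreshes that reference on demand.
; F3 toggles the HUD's debug display, Tab toggles its game menu, and DestroyCurrentSession destroys the session using player controller 0.
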(event `self.ReceiveBeginPlay`
  (`KismetSystemLibrary.Delay` 0.2 :!label _label)
  (bind _asbp_hud (cast `/Game/Blueprints/BP_HUD` (`self.GetHUD`))
    (:`then`
      (set `self.As BP HUD` _asbp_hud))
    (:`CastFailed`
      (goto _label))))

(event `Key|F3`
  (params (Key :type "Key Structure"))
  (:`Pressed`
    (`PS_HUD.ToggleDebug` (`self.As BP HUD`))))

(event `self.DestroyCurrentSession`
  (`DestroySessionCallbackProxy.DestroySession` (`GameplayStatics.GetPlayerController` 0)))

(event `Key|Escape`
  (params (Key :type "Key Structure")))

(event `Key|Tab`
  (params (Key :type "Key Structure"))
  (:`Pressed`
    (`/Game/Blueprints/BP_HUD.Toggle Game Menu 이벤트` (`self.As BP HUD`))))

(fn `Update HUD`
  (bind _asbp_hud (cast `/Game/Blueprints/BP_HUD` (`self.GetHUD`)))
  (set `self.As BP HUD` _asbp_hud))

(fn `UserConstructionScript`)