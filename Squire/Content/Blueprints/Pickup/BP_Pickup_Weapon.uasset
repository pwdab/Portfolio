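; Weapon pickup Blueprint that animates its mesh with a floating, spinning display motion.
; On BeginPlay, the FloatAndRotate timeline adds scaled float and rotate outputs to the mesh's current relative Z and yaw each update, with a fixed roll tilt.
; Overlap and Tick are empty, so no pickup logic appears here.
; Unconnected math computes tilt-compensating X/Y offsets from the stored initial location and capsule height.
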(event `self.ReceiveBeginPlay`
  (bind _mesh (`self.Mesh`))
  (bind (_relativelocation_x _relativelocation_y _relativelocation_z) (`KismetMathLibrary.BreakVector` (`SceneComponent.RelativeLocation` _mesh)))
  (bind (_relativerotation_roll _relativerotation_pitch _relativerotation_yaw) (`KismetMathLibrary.BreakRotator` (`SceneComponent.RelativeRotation` _mesh)))
  (set `self.Initial_Relative_Location` (`SceneComponent.RelativeLocation` (`self.Mesh`)))
  (bind (_direction _float _rotate) (`Timeline|Float and Rotate`)
    (:`Update`
      (`SceneComponent.K2_SetRelativeLocationAndRotation` (`self.Mesh`) (`KismetMathLibrary.MakeVector` 0.0 0.0 (+ (* _float 0.25) _relativelocation_z)) (`KismetMathLibrary.MakeRotator` -10.0 0.0 (+ (* _rotate 1.0) _relativerotation_yaw)) false false))))

(fn `UserConstructionScript`)